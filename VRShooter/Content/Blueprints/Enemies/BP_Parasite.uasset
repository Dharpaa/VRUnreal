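; BP_Parasite is an enemy for the VR player that damages on touch and tracks its own HP.
; On BeginPlay it caches the player pawn and turns its capsule once, in yaw only, to face them.
; Capsule overlap takes 1 HP from the player and sets a collision flag.
; LoseHP feeds CheckDeath, which flags and prints death while HP is zero or above, an apparently inverted test.
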(event OnComponentBeginOverlap(CapsuleComponent)
  (params (OverlappedComponent :type Primitive%20Component%20Object%20Reference) (OtherActor :type Actor%20Object%20Reference) (OtherComp :type Primitive%20Component%20Object%20Reference) (OtherBodyIndex :type Integer) (bFromSweep :type Boolean) (SweepResult :type Hit%20Result%20Structure%20%28by%20ref%29))
  (bind _asbp_vrplayer (Utilities|Casting|CastToBP_VRPlayer OtherActor))
  (Default|LoseHP _asbp_vrplayer 1)
  (Variables|Default|SetIsCollidingPlayer true))

(event EventBeginPlay
  (bind _capsulecomponent (Variables|Collision|GetCapsuleComponent))
  (bind _asbp_vrplayer (Utilities|Casting|CastToBP_VRPlayer (Game|Player|GetPlayerPawn 0)))
  (Variables|Default|SetRefVRPlayer _asbp_vrplayer)
  (Transformation|SetWorldRotation _capsulecomponent (Math|Rotator|MakeRotator 0.0 0.0 (.yaw (Math|Rotator|FindLookatRotation (Transformation|GetWorldLocation _capsulecomponent) (Transformation|GetWorldLocation (Variables|/Script/Engine.Actor|GetRootComponent (Variables|Default|GetRefVRPlayer)))))) false false))

(fn ConstructionScript)

(fn LoseHP
  (params (DmgAmmount :type Integer))
  (Variables|Default|SetHP (- (Variables|Default|GetHP) DmgAmmount))
  (CallFunction|CheckDeath))

(fn CheckDeath
  (if (<= 0 (Variables|Default|GetHP))
    (Variables|Default|SetIsParasiteDead true)
    (Development|PrintString "ParasiteIsDead")))